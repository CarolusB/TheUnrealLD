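; BP_ControlCrane is a prison-level crane control Blueprint that moves its Cube component through input axes.
; Pressing Enter calls Possess on the first player controller with no pawn specified, and releasing it calls UnPossess.
; The CraneMoveX and CraneMoveY axis events share one relative-location offset on X and Y, scaled by Speed and frame delta time.
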(event `Key|Enter`
  (params (Key :type "Key Structure"))
  (bind _returnvalue (`GameplayStatics.GetPlayerController` 0))
  (:`Pressed`
    (`Controller.Possess` _returnvalue null))
  (:`Released`
    (`Controller.UnPossess` _returnvalue)))

(event `InputAxis|CraneMoveX`
  (params (AxisValue :type "Float (single-precision)"))
  (bind _returnvalue (`GameplayStatics.GetWorldDeltaSeconds`))
  (bind _speed (`self.Speed`))
  (`SceneComponent.K2_AddRelativeLocation` (`self.Cube`) (`KismetMathLibrary.MakeVector` (* AxisValue _speed _returnvalue) (* (stale `InputAxis|CraneMoveY` AxisValue) _speed _returnvalue)) false false :!label _label))

(event `InputAxis|CraneMoveY`
  (params (AxisValue :type "Float (single-precision)"))
  (goto _label))

(fn `UserConstructionScript`)